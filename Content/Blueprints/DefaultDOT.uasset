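; DefaultDOT is a damage-over-time actor that drains health from a pawn for a set duration.
; On BeginPlay it computes an end time and starts a looping one-second timer that sends a fixed negative health change to the pawn through AffectHealthMessage.
; Tick checks game time against the end time, then clears the timer and destroys the actor once it expires.
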(event `self.ReceiveTick`
  (params (DeltaSeconds :type "Float (single-precision)"))
  (if (`self.DotStarted`)
    (if (> (`KismetSystemLibrary.GetGameTimeInSeconds`) (`self.EndTime`))
      (`self.CancelDot`))))

(event `self.ReceiveBeginPlay`
  (set `self.EndTime` (+ (`self.Duration`) (`KismetSystemLibrary.GetGameTimeInSeconds`)))
  (`KismetSystemLibrary.K2_SetTimer` null "DotTick" 1.0 true)
  (set `self.DotStarted` true))

(event `DotTick`
  (message `/Game/Blueprints/IDamageable.AffectHealth` (`self.Pawn`) -5.0))

(event `CancelDot`
  (`KismetSystemLibrary.K2_ClearTimer` null "DotTick")
  (`self.K2_DestroyActor`))

(fn `UserConstructionScript`)