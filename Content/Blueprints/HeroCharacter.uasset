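; HeroCharacter is the player character Blueprint, handling its starting weapon, damage and death.
; On BeginPlay it spawns DefaultWeapon attached to GunTemp and saves its own transform to ShadowPainMode as the player spawn point.
; AffectHealth runs CalculateHealth; death triggers a one-time sequence that drops Pawn and WorldDynamic collision, disables input, plays a sound, then after a delay has the game mode respawn the player and destroys the actor.
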(event `self.ReceiveBeginPlay`
  (bind _guntemp (`self.GunTemp`))
  (`|ExecutionSequence`
    (:`then_0`
      (bind _returnvalue (`|SpawnActorFromClass` "/Game/Blueprints/DefaultWeapon.DefaultWeapon_C" (`SceneComponent.K2_GetComponentToWorld` _guntemp) "Undefined" "OverrideRootScale"))
      (bind _output_get (set `self.Weapon` _returnvalue))
      (`self.K2_AttachToComponent` _output_get _guntemp "None" "SnapToTarget" "KeepRelative" "KeepRelative" true))
    (:`then_1`
      (bind _asshadow_pain_mode (cast `/Game/Blueprints/ShadowPainMode` (`GameplayStatics.GetGameMode`)))
      (bind _output_get_2 (set `self.GameMode` _asshadow_pain_mode))
      (set `/Game/Blueprints/ShadowPainMode.PlayerSpawnTransform` (`self.GetTransform`) _output_get_2))))

(event `/Game/Blueprints/IDamageable.AffectHealth`
  (params (Damage :type "Float (single-precision)"))
  (bind _capsulecomponent (`self.CapsuleComponent`))
  (`self.CalculateHealth` Damage)
  (if (`self.IsDead`)
    (`/Engine/EditorBlueprintResources/StandardMacros.DoOnce` false
      (:`Completed`
        (`PrimitiveComponent.SetCollisionResponseToChannel` _capsulecomponent "ECC_Pawn" "ECR_Ignore")
        (`PrimitiveComponent.SetCollisionResponseToChannel` _capsulecomponent "ECC_WorldDynamic" "ECR_Ignore")
        (`self.DisableInput` null)
        (`GameplayStatics.SpawnSoundAttached` "/Game/Audio/Effects/dying_1.dying_1" (`self.Mesh`) "None" (0.0 0.0 0.0) (struct) "KeepRelativeOffset" true)
        (`KismetSystemLibrary.Delay` 2.0)
        (`/Game/Blueprints/ShadowPainMode.RespawnPlayer` (`self.GameMode`))
        (`self.K2_DestroyActor`)))))

(fn `UserConstructionScript`)