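; Enemy character that the player attacks by clicking on it and that is destroyed when killed.
; Capsule click events cast the player to HeroCharacter and pull its weapon trigger, releasing it on mouse release or when the cursor leaves.
; AffectHealth passes damage to CalculateHealth, then destroys the actor if IsDead is set.
; The construction script creates a dynamic material on the mesh to tint BodyColor with EnemyColor.
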(event `self.CapsuleComponent.OnClicked`
  (params (TouchedComponent :type "PrimitiveComponent Object Reference") (ButtonPressed :type "Key Structure" :default "AnyKey"))
  (bind _ashero_character (cast `/Game/Blueprints/HeroCharacter` (`GameplayStatics.GetPlayerCharacter` 0)))
  (`/Game/Blueprints/DefaultWeapon.PullTrigger` (`/Game/Blueprints/HeroCharacter.Weapon` _ashero_character)))

(event `self.CapsuleComponent.OnReleased`
  (params (TouchedComponent :type "PrimitiveComponent Object Reference") (ButtonReleased :type "Key Structure" :default "AnyKey"))
  (bind _ashero_character (cast `/Game/Blueprints/HeroCharacter` (`GameplayStatics.GetPlayerCharacter` 0)))
  (`/Game/Blueprints/DefaultWeapon.ReleaseTrigger` (`/Game/Blueprints/HeroCharacter.Weapon` _ashero_character)))

(event `self.CapsuleComponent.OnEndCursorOver`
  (params (TouchedComponent :type "PrimitiveComponent Object Reference"))
  (bind _ashero_character (cast `/Game/Blueprints/HeroCharacter` (`GameplayStatics.GetPlayerCharacter` 0)))
  (`/Game/Blueprints/DefaultWeapon.ReleaseTrigger` (`/Game/Blueprints/HeroCharacter.Weapon` _ashero_character)))

(event `/Game/Blueprints/IDamageable.AffectHealth`
  (params (Damage :type "Float (single-precision)"))
  (`self.CalculateHealth` Damage)
  (if (`self.IsDead`)
    (`self.K2_DestroyActor`)))

(fn `UserConstructionScript`
  (bind _returnvalue (`PrimitiveComponent.CreateDynamicMaterialInstance` (`self.Mesh`) 0 null))
  (bind _output_get (set `self.DynaMat` _returnvalue))
  (`MaterialInstanceDynamic.SetVectorParameterValue` _output_get "BodyColor" (`self.EnemyColor`)))