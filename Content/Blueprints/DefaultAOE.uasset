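; DefaultAOE is an area-of-effect actor that deals repeated damage to a character inside it.
; On overlap, an IDamageable BaseCharacter is stored, receives Damage through AffectHealthMessage, and a looping one-second timer repeats the hit.
; It tracks only one Character at a time, and any actor ending overlap clears the timer.
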(event `self.ReceiveActorBeginOverlap`
  (params (OtherActor :type "Actor Object Reference"))
  (if (`KismetSystemLibrary.DoesImplementInterface` OtherActor "/Game/Blueprints/IDamageable.IDamageable_C")
    (bind _asbase_character (cast `BaseCharacter` OtherActor))
    (bind _output_get (set `self.Character` _asbase_character))
    (message `/Game/Blueprints/IDamageable.AffectHealth` _output_get (`self.Damage`))
    (`KismetSystemLibrary.K2_SetTimer` null "DoDamage" 1.0 true)))

(event `self.ReceiveActorEndOverlap`
  (params (OtherActor :type "Actor Object Reference"))
  (`KismetSystemLibrary.PrintString` "EndDamage")
  (`KismetSystemLibrary.K2_ClearTimer` null "DoDamage"))

(event `DoDamage`
  (`KismetSystemLibrary.PrintString` "DoDamage")
  (message `/Game/Blueprints/IDamageable.AffectHealth` (`self.Character`) (`self.Damage`)))

(fn `UserConstructionScript`)