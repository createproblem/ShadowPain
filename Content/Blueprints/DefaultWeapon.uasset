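; DefaultWeapon is an automatic laser weapon that fires projectiles while its trigger is held.
; Pulling the trigger fires immediately and starts a looping timer at the rate of fire; releasing it clears the timer and lifts a cooldown after one shot interval.
; Each shot plays a sound on the gun mesh and spawns a projectile at the spawn point.
; The construction script sets a negative Damage value, unused in these graphs.
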(event `PullTrigger`
  (if (not (`self.Cooldown`))
    (set `self.Cooldown` true)
    (`self.Fire`)
    (`KismetSystemLibrary.K2_SetTimer` null "Fire" (/ 1.0 (`self.RoundsPerSecond`)) true)))

(event `ReleaseTrigger`
  (`KismetSystemLibrary.K2_ClearTimer` null "Fire")
  (`KismetSystemLibrary.Delay` (/ 1.0 (`self.RoundsPerSecond`)))
  (set `self.Cooldown` false))

(event `Fire`
  (`GameplayStatics.SpawnSoundAttached` "/Game/Audio/Effects/LaserFire.LaserFire" (`self.GunMesh`))
  (`|SpawnActorFromClass` "/Game/Blueprints/Projectile.Projectile_C" (`SceneComponent.K2_GetComponentToWorld` (`self.ProjectileSpawnPoint`)) "Undefined" "OverrideRootScale"))

(fn `UserConstructionScript`
  (set `self.Damage` -25.0))