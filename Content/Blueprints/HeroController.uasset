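; HeroController is a click-to-move player controller that steers the controlled pawn toward the point under the mouse cursor.
; The SetDestination input opens and closes a gate on Tick, so the cursor is re-traced on the Visibility channel every frame while held.
; MoveToHitLocation ignores hits closer than MinClickDistance, otherwise snaps the pawn's yaw toward the hit, sets RotationCompleted and calls SimpleMoveToLocation.
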(event `self.ReceiveBeginPlay`)

(event `self.ReceiveTick`
  (params (DeltaSeconds :type "Float (single-precision)"))
  (`|ExecutionSequence`
    (:`then_0`
      (`/Engine/EditorBlueprintResources/StandardMacros.Gate` true :!label _label
        (:`Exit`
          (`self.MoveToHitLocation` (`self.GetHitResultUnderCursorByChannel` "TraceTypeQuery1")))))))

(event `InputAction|SetDestination`
  (params (Key :type "Key Structure" :default "AnyKey"))
  (:`Pressed`
    (goto _label :!via `Open`))
  (:`Released`
    (goto _label :!via `Close`)))

(fn `MoveToHitLocation`
  (params (Hit :type "HitResult Structure"))
  (bind (_bblockinghit _binitialoverlap _time _location) (`GameplayStatics.BreakHitResult` Hit))
  (bind _returnvalue (`self.K2_GetPawn`))
  (bind _returnvalue_2 (`self.K2_GetActorLocation` _returnvalue))
  (bind (_returnvalue_roll _returnvalue_pitch _returnvalue_yaw) (`KismetMathLibrary.BreakRotator` (`KismetMathLibrary.FindLookAtRotation` _returnvalue_2 _location)))
  (set `self.RotationCompleted` false)
  (if (>= (`KismetMathLibrary.VSize` (- _returnvalue_2 _location)) (`self.MinClickDistance`))
    (`self.K2_SetActorRotation` _returnvalue (`KismetMathLibrary.MakeRotator` 0.0 0.0 _returnvalue_yaw) false)
    (set `self.RotationCompleted` true)
    (`NavigationSystem.SimpleMoveToLocation` self _location)))

(fn `UserConstructionScript`)