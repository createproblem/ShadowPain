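; HeroLibrary is a small set of helper functions for querying the local player's hero.
; GetPlayerCharacterWeapon casts player 0's character to HeroCharacter and returns its Weapon.
; GetDistanceToCursor runs a complex Visibility trace under the mouse cursor and returns the distance from the controlled pawn to the hit location.
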(fn `GetDistanceToCursor`
  (returns (Distance :type "Float (double-precision)"))
  (bind _returnvalue (`GameplayStatics.GetPlayerController` null))
  (return (`KismetMathLibrary.VSize` (- (`.Location` (`GameplayStatics.BreakHitResult` (`PlayerController.GetHitResultUnderCursorByChannel` _returnvalue "TraceTypeQuery1" true))) (`Actor.K2_GetActorLocation` (`Controller.K2_GetPawn` _returnvalue))))))

(fn `GetPlayerCharacterWeapon`
  (returns (Weapon :type "/Game/Blueprints/DefaultWeapon Object Reference"))
  (bind _ashero_character (cast `/Game/Blueprints/HeroCharacter` (`GameplayStatics.GetPlayerCharacter` null)))
  (return (`/Game/Blueprints/HeroCharacter.Weapon` _ashero_character)))